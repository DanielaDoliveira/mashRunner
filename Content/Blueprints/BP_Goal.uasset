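; BP_Goal is the finish goal of a lane in the runner game, declaring that lane the winner when a runner reaches it.
; A box collision overlap with BP_Runner fires TriggerGoal through a DoOnce, so each goal triggers only once.
; TriggerGoal swaps the Paper2D sprite to a ripped version and passes its LaneIndex to AnnouceWinner on the GM_Runner game mode cached at BeginPlay.
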(event `self.ReceiveBeginPlay`
  (bind _asgm_runner (cast `/Game/Blueprints/GM_Runner` (`GameplayStatics.GetGameMode`)))
  (set `self.GameMode` _asgm_runner))

(event `self.BoxCollision.OnComponentBeginOverlap`
  (params (OverlappedComponent :type "PrimitiveComponent Object Reference") (OtherActor :type "Actor Object Reference") (OtherComp :type "PrimitiveComponent Object Reference") (OtherBodyIndex :type Integer) (bFromSweep :type Boolean) (SweepResult :type "HitResult Structure (by ref)"))
  (cast `/Game/Blueprints/BP_Runner` OtherActor)
  (`/Engine/EditorBlueprintResources/StandardMacros.DoOnce` false
    (:`Completed`
      (`self.TriggerGoal`))))

(fn `TriggerGoal`
  (`PaperSpriteComponent.SetSprite` (`self.PaperSprite`) "/Game/PaperAssets/Goal/T_Goal_Ripped_Sprite.T_Goal_Ripped_Sprite")
  (`/Game/Blueprints/GM_Runner.AnnouceWinner` (`self.GameMode`) (`self.LaneIndex`)))

(fn `UserConstructionScript`)